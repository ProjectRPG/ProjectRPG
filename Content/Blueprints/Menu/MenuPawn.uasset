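; Menu pawn that presents the menu as a book whose pages turn through animations when left or right buttons are clicked.
; Each click passes the current page and a direction enum to UpdateCurrentAnim, whose nested switches pick an animation and next page for TurnPage to play on Book.
; Only one transition per direction is defined, both using the same animation, and the CurrentPage update is unwired, so the page state never advances.
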(event `self.RightButton.OnClicked`
  (params (TouchedComponent :type "PrimitiveComponent Object Reference"))
  (set `self.Direction` "NewEnumerator1")
  (bind (_newanimation _newpage) (`self.UpdateCurrentAnim` (`self.CurrentPage`) (`self.Direction`) :!label _label))
  (`self.TurnPage` _newanimation))

(event `self.LeftButton.OnClicked`
  (params (TouchedComponent :type "PrimitiveComponent Object Reference"))
  (set `self.Direction` "NewEnumerator0")
  (goto _label))

(fn `TurnPage`
  (params (Animation :type "AnimSequence Object Reference"))
  (`SkeletalMeshComponent.PlayAnimation` (`self.Book`) Animation false))

(fn `UpdateCurrentAnim`
  (params (CurrentPage :type "/Game/Blueprints/Menu/CurrentPageState Enum" :default "NewEnumerator0") (Direction :type "/Game/Blueprints/Menu/PageDirection Enum" :default "NewEnumerator0"))
  (returns (NewAnimation :type "AnimSequence Object Reference") (NewPage :type "/Game/Blueprints/Menu/CurrentPageState Enum"))
  (bind _variable (`|LocalVariable`))
  (bind _variable_2 (`|LocalVariable`))
  (switch `/Game/Blueprints/Menu/PageDirection` Direction
    (:`NewEnumerator0`
      (switch `/Game/Blueprints/Menu/CurrentPageState` CurrentPage
        (:`NewEnumerator0`
          (`|AssignmentStatement` _variable_2 "NewEnumerator1")
          (`|AssignmentStatement` _variable "/Game/Animations/Book/About_Into_Anim.About_Into_Anim"))))
    (:`NewEnumerator1`
      (switch `/Game/Blueprints/Menu/CurrentPageState` CurrentPage
        (:`NewEnumerator1`
          (`|AssignmentStatement` _variable_2 "NewEnumerator0")
          (`|AssignmentStatement` _variable "/Game/Animations/Book/About_Into_Anim.About_Into_Anim")))))
  (return _variable _variable_2))

(fn `UserConstructionScript`)